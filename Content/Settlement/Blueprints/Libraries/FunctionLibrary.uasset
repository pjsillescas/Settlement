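; Function library of shared helpers for a settlement-building game.
; Placement helpers snap values to a grid, find the cursor's world position (line trace when building, otherwise deprojected mouse location with non-negative Z), fit collision boxes to mesh bounds and compute actor height above ground.
; A clock helper advances time on a 24-unit cycle and outputs day rollover.
; The HUD lerp helper has zero alpha, so it returns the current location.
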(fn GridSnap
  (params (AxisIn :type Float%20%28single-precision%29) (GridSize :type Integer))
  (return (Math|Conversions|ToFloat(Integer) (* (Math|Float|Floor (/ (+ AxisIn (Math|Conversions|ToFloat(Integer) (/ GridSize 2))) (Math|Conversions|ToFloat(Integer) GridSize))) GridSize))))

(fn SetCursorWorldPosition
  (params (Controller :type Player%20Controller%20Object%20Reference) (SightDistance :type Float%20%28single-precision%29) (bIsBuilding :type Boolean))
  (bind (_worldlocation _worlddirection) (Game|Player|ConvertMouseLocationToWorldSpace Controller))
  (bind (_x _y _z) (Math|Vector|BreakVector _worldlocation))
  (if bIsBuilding
    (bind _outhit (Collision|LineTraceByChannel 0 _worldlocation (+ _worldlocation (* _worlddirection SightDistance)) "TraceTypeQuery3" false 0 "ForOneFrame"))
    (if (!= (.HitActor (Collision|BreakHitResult _outhit)) 0)
      (return (.Location (Collision|BreakHitResult _outhit))))
    (else
      (return (Math|Vector|MakeVector _x _y (Math|Float|Clamp(Float) _z 0.0 1e+08))))))

(fn SetClockwork
  (params (DeltaSeconds :type Float%20%28single-precision%29) (TimeUnit :type Float%20%28single-precision%29) (ClockworkIn :type Float%20%28single-precision%29))
  (bind _returnvalue (/ DeltaSeconds TimeUnit))
  (bind _returnvalue_2 (+ _returnvalue ClockworkIn))
  (bind (_remainder _returnvalue_3) (Math|Float|Division(WholeandRemainder) _returnvalue_2 24.0))
  (return _remainder _returnvalue_3))

(fn AdjustCollisionBoxtoMesh
  (params (CollisionBox :type Box%20Component%20Object%20Reference) (Mesh :type Static%20Mesh%20Component%20Object%20Reference))
  (bind _min (Components|StaticMesh|GetLocalBounds Mesh))
  (Components|Box|SetBoxExtent CollisionBox (Math|Vector|MakeVector (- (Math|Float|Absolute(Float) (.x _min)) 2e+01) 98.0 1e+01) true)
  (Transformation|SetRelativeLocation CollisionBox (Math|Vector|MakeVector 0.0 (+ (Math|Float|Absolute(Float) (.y _min)) 98.0) 1e+01) false false)
  (return))

(fn HUDLerpLocation
  (params (CurrentLocation :type Vector) (Destination :type Vector))
  (bind _returnvalue (Math|Vector|Lerp(Vector) CurrentLocation Destination 0.0))
  (return (Math|Vector|MakeVector (.x _returnvalue) (.y _returnvalue) (.Z (Math|Vector|BreakVector CurrentLocation)))))

(fn GetActorZOffset
  (params (Actor :type Actor%20Object%20Reference) (Ground :type Actor%20Object%20Reference))
  (return (+ (Math|Conversions|ToFloat(Integer) (Math|Float|Truncate (.z (.BoxExtent (Collision|GetActorBounds Actor false))))) (.z (Transformation|GetActorLocation Ground)))))