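; SettlementCharacterNPC is an NPC character Blueprint for the Settlement game, with a configurable body color.
; Its construction script runs the parent's, then creates a dynamic instance of M_UE4Man_Body on mesh slot 0 and applies the Color variable to its body color parameter.
; On BeginPlay it casts player controller 0 to SettlementPlayerController and caches the reference, with no further gameplay logic here.
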(event EventBeginPlay
  (bind _assettlement_player_controller (Utilities|Casting|CastToSettlementPlayerController (Game|GetPlayerController 0)))
  (Variables|Default|SetPlayerController _assettlement_player_controller))

(event Collision|EventActorBeginOverlap
  (params (OtherActor :type Actor%20Object%20Reference)))

(event EventTick
  (params (DeltaSeconds :type Float%20%28single-precision%29)))

(fn ConstructionScript
  (|CallParentFunction)
  (bind _returnvalue (Rendering|Material|CreateDynamicMaterialInstance (Variables|Character|GetMesh) 0 "/Game/Mannequin/Character/Materials/M_UE4Man_Body.M_UE4Man_Body" :!class /Script/Engine.PrimitiveComponent))
  (bind _output_get (Variables|Default|SetNPCMaterialInstance _returnvalue))
  (Rendering|Material|SetVectorParameterValue _output_get (Variables|Configuration|GetBodyColorName) (Variables|Info|GetColor) :!class /Script/Engine.MaterialInstanceDynamic))