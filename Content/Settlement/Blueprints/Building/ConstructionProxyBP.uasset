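; Placeholder actor for a settlement building under construction, showing the display mesh in a proxy material with a collision box fitted to it.
; Each tick it advances a work clock using the game-state time unit divided by active worker count, so more workers build faster.
; Game speed updates are bound through the game state.
; When work time reaches construction time, it frees and unhides its workers, then destroys itself shortly after.
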(event Custom|AdjustTime
  (params (TimeUnit :type Float%20%28single-precision%29))
  (Variables|Default|SetTimeUnit TimeUnit))

(event EventBeginPlay
  (CallFunction|Initialize))

(event Collision|EventActorBeginOverlap
  (params (OtherActor :type Actor%20Object%20Reference)))

(event EventTick
  (params (DeltaSeconds :type Float%20%28single-precision%29))
  (Utilities|TickMacro DeltaSeconds))

(fn ConstructionScript
  (bind _staticmesh (Variables|Default|GetStaticMesh))
  (Components|StaticMesh|SetStaticMesh _staticmesh (Variables|Default|GetDisplayMesh))
  (Rendering|Material|SetMaterial _staticmesh 0 "/Game/Settlement/Materials/MConstructionProxy.MConstructionProxy")
  (CallFunction|AdjustCollisionBoxtoMesh (Variables|Default|GetCollisionBox) (Variables|Default|GetStaticMesh))
  (Variables|Default|SetWorkers (Utilities|Array|MakeArray 0)))

(fn ReleaseWorker
  (params (Worker :type Settlement%20Character%20NPC%20Object%20Reference%20%28by%20ref%29))
  (if (> (Utilities|Array|FindItem (Variables|Default|GetActiveWorkers) Worker) -1)
    (bind _returnvalue (Utilities|Array|RemoveItem (Variables|Default|GetActiveWorkers) 0))
    (return _returnvalue)
    (else
      (return false))))

(fn SetConstructionTime
  (params (ConstructionTime :type Float%20%28single-precision%29))
  (Variables|Default|SetConstructionTime ConstructionTime)
  (return))

(fn AddWorker
  (params (Worker :type Settlement%20Character%20NPC%20Object%20Reference%20%28by%20ref%29))
  (Utilities|Array|Add (Variables|Default|GetActiveWorkers) Worker)
  (return))

(fn GetWorkForce
  (return (Utilities|Array|Length (Variables|Default|GetActiveWorkers))))

(fn DoWork
  (bind _activeworkers (CallFunction|GetWorkForce))
  (bind _returnvalue (Math|Conversions|ToFloat(Integer) _activeworkers))
  (if (> _returnvalue 0.0)
    (bind _output_get (Variables|Default|SetClockwork (.ClockworkOut (CallFunction|SetClockwork (Variables|Default|GetDelta) (/ (Variables|Default|GetTimeUnit) _returnvalue) (Variables|Default|GetClockwork)))))
    (Variables|Default|SetWorkTimeSpent _output_get)
    (return)
    (else
      (return))))

(fn ConstructionComplete
  (if (> (Math|Conversions|ToFloat(Integer) (CallFunction|GetWorkForce)) 0.0)
    (for _array_element (Variables|Default|GetActiveWorkers)
      (LocalVariables|SetLocalWorker _array_element)
      (Utilities|FlowControl|Sequence
        (:then_0
          (Default|SetIsBusy (LocalVariables|GetLocalWorker) false))
        (:then_1
          (Rendering|SetActorHiddenInGame (LocalVariables|GetLocalWorker) false))))
    (Variables|Default|SetActiveWorkers (Utilities|Array|MakeArray 0))
    (return)
    (else
      (return))))

(fn Initialize
  (bind _assettlement_game_state (Utilities|Casting|CastToSettlementGameState (Game|GetGameState)))
  (bind _output_get (Variables|Default|SetGameStateRef _assettlement_game_state))
  (EventDispatchers|BindEventtoUpdateGameSpeed _output_get (EventDispatchers|CreateEvent :!event Custom|AdjustTime))
  (bind _timeunit (Default|GetCurrentTimeUnit (Variables|Default|GetGameStateRef)))
  (Variables|Default|SetTimeUnit _timeunit)
  (Variables|Default|SetPlayerControllerRef (.AsSettlement%20Player%20Controller (Utilities|Casting|CastToSettlementPlayerController (Game|GetPlayerController 0)))))