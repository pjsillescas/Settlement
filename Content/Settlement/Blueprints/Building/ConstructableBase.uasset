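; Base Blueprint for constructable buildings in the settlement system, serving as a data holder with no behavior of its own.
; It stores a proxy, a display mesh, a construction time and a controller reference, each exposed through a plain getter and setter function.
; The event graph and construction script are empty, so this file contains no construction or placement logic.
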(event EventBeginPlay)

(event Collision|EventActorBeginOverlap
  (params (OtherActor :type Actor%20Object%20Reference)))

(event EventTick
  (params (DeltaSeconds :type Float%20%28single-precision%29)))

(fn ConstructionScript)

(fn GetProxy
  (return (Variables|Default|GetProxy)))

(fn SetProxy
  (params (Proxy :type Construction%20Proxy%20BP%20Class%20Reference))
  (Variables|Default|SetProxy Proxy)
  (return))

(fn GetDisplayMesh
  (return (Variables|Default|GetDisplayMesh)))

(fn SetDisplayMesh
  (params (DisplayMesh :type Static%20Mesh%20Object%20Reference))
  (Variables|Default|SetDisplayMesh DisplayMesh)
  (return))

(fn GetConstructionTime
  (return (Variables|Default|GetConstructionTime)))

(fn SetConstructionTime
  (params (ConstructionTime :type Float%20%28single-precision%29))
  (Variables|Default|SetConstructionTime ConstructionTime)
  (return))

(fn GetControllerRef
  (return (Variables|Default|GetControllerRef)))

(fn SetControllerRef
  (params (ControllerRef :type Settlement%20Player%20Controller%20Object%20Reference))
  (Variables|Default|SetControllerRef ControllerRef)
  (return))