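; Placement preview actor for build mode, showing a translucent-style ghost of the chosen building at the grid-snapped cursor position.
; Construct briefly spawns the building class to read its mesh, proxy and work hours, then activates the ghost with pawn-derived stepped yaw.
; Gated Tick moves it and swaps to an error material on actor overlap or excessive slope, measured by corner and center traces.
; GetConstructionData exposes the placement; KillGhost resets it.
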(event Custom|OnSpawn
  (params (DisplayMesh :type Static%20Mesh%20Object%20Reference) (BuildingClass :type Constructable%20Base%20Class%20Reference) (ConstructionProxy :type Construction%20Proxy%20BP%20Class%20Reference) (WorkHours :type Float%20%28single-precision%29))
  (bind _arrow (Variables|Default|GetArrow))
  ;[1 1 1] Event On Spawn
  (if (not (Variables|Default|GetbIsActive))
    (Variables|Default|SetDisplayMesh DisplayMesh)
    (Variables|Default|SetBuildingClass BuildingClass)
    (Variables|Default|SetConstructionProxy ConstructionProxy)
    (Variables|Default|SetWorkHoursRequired WorkHours)
    (Variables|Default|SetbIsActive true)
    (Default|SetBuildModeActive (Variables|Default|GetControllerRef) true)
    (Components|StaticMesh|SetStaticMesh (Variables|Default|GetGhostMesh) (Variables|Default|GetDisplayMesh))
    (CallFunction|OpenTickGate)
    (CallFunction|SetMaterial (not (Variables|Default|GetbIsOverlapping)))
    (bind _output_get (Variables|Default|SetExtent (.BoxExtent (Collision|GetComponentBounds 0))))
    (Transformation|SetRelativeLocation _arrow (Math|Vector|MakeVector 0.0 (.Y (Math|Vector|BreakVector _output_get)) 0.0) false false)
    (Development|SetHiddeninGame _arrow false false)
    (CallFunction|AdjustCollisionBoxtoMesh (Variables|Default|GetCollisionBox) (Variables|Default|GetGhostMesh))
    (bind _returnedrotation (CallFunction|SetInitialRotation))
    (Transformation|SetActorRotation (Math|Rotator|MakeRotator 0.0 0.0 (+ _returnedrotation 9e+01)))))

(event Custom|SetMaterial
  (params (bIsError :type Boolean))
  ;[1 1 1] Set Material
  (Utilities|SetMaterialMacro bIsError))

(event Custom|KillGhost
  ;[1 1 1] Event Kill Ghost
  (Variables|Default|SetBuildingClass 0)
  (Variables|Default|SetConstructionProxy 0)
  (CallFunction|CloseTickGate)
  (Variables|Default|SetDisplayMesh 0)
  (Variables|Default|SetbIsActive false)
  (Default|SetBuildModeActive (Variables|Default|GetControllerRef) false)
  (Components|StaticMesh|SetStaticMesh (Variables|Default|GetGhostMesh) (Variables|Default|GetDisplayMesh))
  (Transformation|SetActorRotation "0, 0, 0")
  (Development|SetHiddeninGame (Variables|Default|GetArrow) true false))

(event Custom|OpenTickGate
  ;[1 1 1] Event Tick
  (Utilities|FlowControl|Gate true) ; enters at Open
)

(event Custom|CloseTickGate
  ;[1 1 1] Event Tick
  (Utilities|FlowControl|Gate true) ; enters at Close
)

(event EventBeginPlay)

(event Collision|EventActorBeginOverlap
  (params (OtherActor :type Actor%20Object%20Reference)))

(event EventTick
  (params (DeltaSeconds :type Float%20%28single-precision%29))
  ;[1 1 1] Event Tick
  (Utilities|FlowControl|Gate true
    (:Exit
      (Utilities|TickMacro))))

(event EventConstruct
  (params (Constructable :type Constructable%20Base%20Class%20Reference))
  ;[1 1 1] Event Construct
  (bind _returnvalue (Game|SpawnActorfromClass Constructable (Math|Transform|MakeTransform (Variables|Default|GetCursorWorldPosition)) "Undefined" 0 (Variables|Default|GetControllerRef) 0))
  (Utilities|FlowControl|Sequence
    (:then_0
      (CallFunction|KillGhost)
      (CallFunction|OnSpawn (Default|GetDisplayMesh _returnvalue) Constructable (Default|GetProxy _returnvalue) (Default|GetConstructionTime _returnvalue)))
    (:then_1
      (Actor|DestroyActor _returnvalue))))

(fn ConstructionScript)

(fn GetVectors
  (bind _returnvalue (Transformation|GetActorRotation))
  (return (Transformation|GetActorLocation) (Math|Vector|GetForwardVector _returnvalue) (Math|Vector|GetRightVector _returnvalue)))

(fn SlopeTrace
  (params (TraceLocation :type Vector))
  (bind _localdifference (LocalVariables|GetLocalDifference))
  (bind _outhit (Collision|LineTraceByChannel (+ TraceLocation _localdifference) (- TraceLocation _localdifference) (LocalVariables|GetLocalTraceChannel) false 0 "ForOneFrame"))
  (return (- (.z (Transformation|GetActorLocation)) (.Z (Math|Vector|BreakVector (.ImpactPoint (Collision|BreakHitResult _outhit)))))))

(fn SetGridSnapVector
  (bind _cursorworldposition (Variables|Default|GetCursorWorldPosition))
  (bind _gridsize (Variables|Default|GetGridSize))
  (bind (_x _y _z) (Math|Vector|BreakVector _cursorworldposition))
  (return (Math|Vector|MakeVector (CallFunction|GridSnap _x _gridsize) (CallFunction|GridSnap _y _gridsize) (CallFunction|GridSnap _z _gridsize))))

(fn GetConstructionData
  (return (Variables|Default|GetBuildingClass) (Variables|Default|GetConstructionProxy) (Math|Transform|MakeTransform (Transformation|GetActorLocation) (Transformation|GetActorRotation) "0.500000,0.500000,0.500000") (Variables|Default|GetDisplayMesh) (Variables|Default|GetWorkHoursRequired)))

(fn CheckOverlap
  (return (> (Utilities|Array|Length (Collision|GetOverlappingActors "/Script/Engine.Actor" :!class /Script/Engine.Actor)) 0)))

(fn CalculateSlope
  (bind (_location _forward) (CallFunction|GetVectors))
  (bind _location_2 (CallFunction|GetVectors))
  (bind _extent (Variables|Default|GetExtent))
  (bind _differences (LocalVariables|GetDifferences))
  (bind _maxdifferences (LocalVariables|GetMaxDifferences))
  (bind _differences_2 (LocalVariables|GetDifferences))
  (bind _tracedisplacement (Variables|Default|GetTraceDisplacement))
  (bind _returnvalue (Math|Vector|MakeVector (.x _location_2) (.y _location_2) (.z _location_2)))
  (bind (_indexofminvalue _minvalue) (Math|Float|MinOfFloatArray _differences_2))
  (bind (_indexofmaxvalue _maxvalue) (Math|Float|MaxOfFloatArray _differences_2))
  (bind (_x _y) (Math|Vector|BreakVector _extent))
  (Utilities|FlowControl|Sequence
    (:then_0
      (Utilities|FlowControl|Sequence
        (:then_0
          (Utilities|CalculateDifference 1.0 1.0 _differences))
        (:then_1
          (Utilities|CalculateDifference -1.0 1.0 _differences))
        (:then_2
          (Utilities|CalculateDifference 1.0 -1.0 _differences))
        (:then_3
          (Utilities|CalculateDifference -1.0 -1.0 _differences))
        (:then_4
          (Utilities|CalculateDifference 0.0 0.0 _differences))))
    (:then_1
      (for _array_element (LocalVariables|GetDifferences)
        (LocalVariables|SetNewLocalVar_0 (Utilities|String|Append (Utilities|String|ToString(Float) _array_element) "," (LocalVariables|GetNewLocalVar_0))))
      (Development|PrintString (LocalVariables|GetNewLocalVar_0))
      (if (and (> _indexofminvalue -1) (> _indexofmaxvalue -1))
        (bind (_outhit _returnvalue_2) (Collision|BoxTraceByChannel (+ _location _tracedisplacement) (- _forward _tracedisplacement) (Math|Vector|MakeVector _x _y 1.0) "0, 0, 0" "TraceTypeQuery1" false 0 "None"))
        (if _returnvalue_2
          (Development|PrintString (Utilities|String|ToString(Vector) _returnvalue))
          (Transformation|SetActorLocation _returnvalue false false))))
    (:then_2
      (return (or (> (Math|Float|Absolute(Float) _minvalue) _maxdifferences) (> (Math|Float|Absolute(Float) _maxvalue) _maxdifferences))))))

(fn SetInitialRotation
  (bind _controllerref (Variables|Default|GetControllerRef))
  (bind _rotationrate (Default|GetBuildingRotationRate _controllerref))
  (bind _returnvalue (Pawn|GetControlledPawn _controllerref))
  (bind _returnvalue_2 (VehicleSound|GetRootComponent _returnvalue))
  (bind _returnvalue_3 (Transformation|GetWorldRotation _returnvalue_2))
  (bind _yaw (Math|Rotator|BreakRotator _returnvalue_3))
  (if (and (< _yaw (* _rotationrate -1.0)) (> _yaw _rotationrate))
    (return 0.0)
    (else
      (return (* (.ReturnValue (Math|Float|Division(WholeandRemainder) (Math|Conversions|ToFloat(Integer) (Math|Float|Round _yaw)) _rotationrate)) _rotationrate)))))

(fn GetCursorPosition
  (return (Variables|Default|GetCursorWorldPosition)))

(fn SetCursorPosition
  (params (CursorWorldPosition :type Vector))
  (Variables|Default|SetCursorWorldPosition CursorWorldPosition)
  (return))