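; SettlementCharacter is a character Blueprint that adds double jump and a placeholder interaction input.
; The Jump input feeds DoDoubleJump, whose DoN counter allows two presses: a normal jump, then a launch that overrides Z velocity with DoubleJumpHeight.
; Landing resets the counter.
; The Interaction input only prints a message.
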(event EventBeginPlay)

(event Collision|EventActorBeginOverlap
  (params (OtherActor :type Actor%20Object%20Reference)))

(event EventTick
  (params (DeltaSeconds :type Float%20%28single-precision%29)))

(event EventOnLanded
  (params (Hit :type Hit%20Result%20Structure%20%28by%20ref%29))
  ;[1 1 1] Double Jump
  (Utilities|DoDoubleJump) ; enters at Reset
)

(event Input|ActionEvents|InputActionInteraction
  (params (Key :type Key%20Structure :default "AnyKey"))
  (:Pressed
    (Development|PrintString "Interacting")))

(event Input|ActionEvents|InputActionJump
  (params (Key :type Key%20Structure :default "AnyKey"))
  ;[1 1 1] Double Jump
  (:Pressed
    (Utilities|DoDoubleJump)))

(fn ConstructionScript
  (|CallParentFunction))